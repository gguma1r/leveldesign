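; AI pawn Blueprint that patrols a looping route of waypoint actors.
; On BeginPlay it starts an AI MoveTo toward the current entry in the Waypoint array.
; Each successful arrival increments the index, wraps it to zero past the last entry and calls the follow event again.
; Only the success result is handled, so a failed move does not trigger another.
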(event `self.ReceiveBeginPlay`
  (`self.Follow_waypoint`))

(event `Follow_waypoint`
  (`|AIMoveTo` self (0.0 0.0 0.0) (`|GetArrayItem` (`self.waypoint`) (`self.Cuurent_waypoint`))
    (:`OnSuccess`
      (`/Engine/EditorBlueprintResources/StandardMacros.IncrementInt` (`self.Cuurent_waypoint`)
        (:`  `
          (if (>= (`self.Cuurent_waypoint`) (`KismetArrayLibrary.Array_Length` (`self.waypoint`)))
            (set `self.Cuurent_waypoint` 0))
          (`self.Follow_waypoint`))))))

(fn `UserConstructionScript`)